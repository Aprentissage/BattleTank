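; Tank Blueprint that wires player input to driving, camera aiming and firing.
; On BeginPlay it hands the barrel and turret to the TankAiming component and both tracks to TankMouvement.
; Driving works either by per-track throttle or by forward and turn intents sent to TankMouvement.
; Aim axes rotate the azimuth gimbal (yaw) and spring arm (pitch) scaled by delta time, and Fire calls TankAiming.
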(event `self.ReceiveBeginPlay`
  (`TankAimingComponent.initialise` (`self.TankAiming`) (`self.TankBarrel1`) (`self.TankTurret1`))
  (`TankMouvementComponent.initialise` (`self.TankMouvement`) (`self.LeftTrack`) (`self.rightTrack`)))

(event `InputAxis|Left Track Throttle`
  (params (AxisValue :type "Float (single-precision)"))
  ;[1 1 1] Mouvement input binding
  (`TankTrack.SetThrottle` (`self.LeftTrack`) AxisValue))

(event `InputAxis|Right Track Throttle`
  (params (AxisValue :type "Float (single-precision)"))
  ;[1 1 1] Mouvement input binding
  (`TankTrack.SetThrottle` (`self.rightTrack`) AxisValue))

(event `InputAxis|GoForeward`
  (params (AxisValue :type "Float (single-precision)"))
  ;[1 1 1] Mouvement input binding
  (`TankMouvementComponent.IntendMoveForward` (`self.TankMouvement`) AxisValue))

(event `InputAxis|AimAzimuth`
  (params (AxisValue :type "Float (single-precision)"))
  ;[1 1 1] Aiming input binding
  (`SceneComponent.K2_AddLocalRotation` (`self.AzimuthGimbal`) (`KismetMathLibrary.MakeRotator` 0.0 0.0 (* AxisValue (`GameplayStatics.GetWorldDeltaSeconds`) 100.0)) false false))

(event `InputAxis|GoBackward`
  (params (AxisValue :type "Float (single-precision)"))
  ;[1 1 1] Mouvement input binding
  (`TankMouvementComponent.IntendMoveForward` (`self.TankMouvement`) AxisValue))

(event `InputAxis|AimElevation`
  (params (AxisValue :type "Float (single-precision)"))
  ;[1 1 1] Aiming input binding
  (`SceneComponent.K2_AddLocalRotation` (`self.SpringArm`) (`KismetMathLibrary.MakeRotator` 0.0 (* AxisValue (`GameplayStatics.GetWorldDeltaSeconds`) 100.0)) false false))

(event `InputAxis|GoRight`
  (params (AxisValue :type "Float (single-precision)"))
  ;[1 1 1] Mouvement input binding
  (`TankMouvementComponent.IntendTurnRight` (`self.TankMouvement`) AxisValue))

(event `InputAxis|GoLeft`
  (params (AxisValue :type "Float (single-precision)"))
  ;[1 1 1] Mouvement input binding
  (`TankMouvementComponent.IntendTurnRight` (`self.TankMouvement`) AxisValue))

(event `InputAction|Fire`
  (params (Key :type "Key Structure"))
  ;[1 1 1] Aiming input binding
  (:`Pressed`
    (`TankAimingComponent.fire` (`self.TankAiming`))))

(fn `UserConstructionScript`)